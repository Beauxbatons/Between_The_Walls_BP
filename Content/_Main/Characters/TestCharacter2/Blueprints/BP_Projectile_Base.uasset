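; BP_Projectile_Base is a projectile Blueprint that damages BP_TestCharacter2 on overlap.
; Its overlap event prints the other actor's name, casts it to that character, subtracts a fixed amount directly from its Health and prints the result.
; The graph does not destroy the projectile or use the damage system, and its Hit, BeginPlay, Tick and construction logic are empty.
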(event EventBeginPlay)

(event Collision|EventActorBeginOverlap
  (params (OtherActor :type Actor%20Object%20Reference))
  (Development|PrintString (Utilities|GetDisplayName OtherActor))
  (bind _asbp_test_character_2 (Utilities|Casting|CastToBP_TestCharacter2 OtherActor))
  (Variables|/Game/_Main/Characters/TestCharacter2/Blueprints/BP_TestCharacter2.BP_TestCharacter2_C|SetHealth _asbp_test_character_2 (- (Variables|/Game/_Main/Characters/TestCharacter2/Blueprints/BP_TestCharacter2.BP_TestCharacter2_C|GetHealth _asbp_test_character_2) 1e+01))
  (Development|PrintString (Utilities|String|ToString(Float) (Variables|/Game/_Main/Characters/TestCharacter2/Blueprints/BP_TestCharacter2.BP_TestCharacter2_C|GetHealth _asbp_test_character_2))))

(event EventTick
  (params (DeltaSeconds :type Float%20%28single-precision%29)))

(event Collision|EventHit
  (params (MyComp :type Primitive%20Component%20Object%20Reference) (Other :type Actor%20Object%20Reference) (OtherComp :type Primitive%20Component%20Object%20Reference) (bSelfMoved :type Boolean) (HitLocation :type Vector :default "0, 0, 0") (HitNormal :type Vector :default "0, 0, 0") (NormalImpulse :type Vector :default "0, 0, 0") (Hit :type Hit%20Result%20Structure%20%28by%20ref%29)))

(fn ConstructionScript)