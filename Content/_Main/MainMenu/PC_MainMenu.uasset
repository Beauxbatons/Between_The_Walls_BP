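; Main menu player controller that sets up the local player's name and avatar on BeginPlay.
; After a short delay it reads the Steam persona name and requests the friend avatar when the Steam subsystem is present.
; Without Steam, or if the avatar fails and the name is empty, it uses a random name and image from the GameInstance.
; The resulting PlayerInfo is saved through GameInstance messages, followed by a main menu player-info message.
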(event EventBeginPlay
  (bind _returnvalue (Game|GetGameInstance))
  (bind _returnvalue_2 (Game|GetGameInstance))
  (bind _returnvalue_3 (Game|GetGameInstance))
  (Utilities|FlowControl|Delay 0.2)
  (if (Class|AdvancedSessionsLibrary|HasOnlineSubsystem "steam")
    (bind _returnvalue_4 (Class|AdvancedSteamFriendsLibrary|GetSteamPersonaName (Class|AdvancedSessionsLibrary|GetUniqueNetID self)))
    (Variables|Default|SetPlayerName (Utilities|Text|ToText(String) _returnvalue_4))
    (bind _returnvalue_5 (Class|AdvancedSteamFriendsLibrary|GetSteamFriendAvatar (Class|AdvancedSessionsLibrary|GetUniqueNetID self) "SteamAvatar_Medium")
      (:OnSuccess
        (bind _structout (Utilities|Struct|SetmembersinS_PlayerInfo (Variables|Default|GetPlayerInfo) (Variables|Default|GetPlayerName) _returnvalue_5))
        (Class|BPIGameInstance|SavePlayerInfo(Message) _returnvalue_2 _structout)
        (Class|BPIGameInstance|MainMenuPlayerInfo(Message) _returnvalue_2))
      (:OnFailure
        (if (Utilities|Text|TextIsEmpty (Variables|Default|GetPlayerName))
          (bind (_name _image) (Class|BPIGameInstance|GetRandomNameandImage(Message) (Game|GetGameInstance)))
          (bind _structout_2 (Utilities|Struct|SetmembersinS_PlayerInfo (Variables|Default|GetPlayerInfo) _name _image))
          (Class|BPIGameInstance|SavePlayerInfo(Message) _returnvalue_3 _structout_2)
          (Class|BPIGameInstance|MainMenuPlayerInfo(Message) _returnvalue_3))))
    (else
      (bind (_name_2 _image_2) (Class|BPIGameInstance|GetRandomNameandImage(Message) (Game|GetGameInstance)))
      (bind _structout_3 (Utilities|Struct|SetmembersinS_PlayerInfo (Variables|Default|GetPlayerInfo) _name_2 _image_2))
      (Class|BPIGameInstance|SavePlayerInfo(Message) _returnvalue _structout_3)
      (Class|BPIGameInstance|MainMenuPlayerInfo(Message) _returnvalue))))

(fn ConstructionScript)